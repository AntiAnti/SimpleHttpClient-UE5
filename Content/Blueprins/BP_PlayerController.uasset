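; Player controller that turns a typed prompt into a spoken reply from a talking head, using local LLM and TTS servers.
; It creates the main UI and drives a state machine that gates requests and updates the status widget.
; HTTP responses chain an OpenAI-style chat request into voice synthesis with a reference WAV, then Runtime Audio Importer loads the result for SpeakingHead.
; Request errors print a state-specific message and reset to Idle.
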(event `SetGenerationState`
  (params (NewState :type "/Game/Blueprins/E_State Enum" :default "NewEnumerator0"))
  ;[1 1 1] Set generation state and update UI
  (bind _output_get (set `self.State` NewState))
  (`/Game/UI/W_Main.UpdateStateWidget` (`self.MainUI`) _output_get))

(event `self.ReceiveBeginPlay`
  (bind _returnvalue (subsystem `HTTPSubsystem`))
  (`|ExecutionSequence`
    (:`then_0`
      ;[1 1 1] Create UI
      (bind _returnvalue_2 (`|CreateWidget` "/Game/UI/W_Main.W_Main_C" self))
      (bind _output_get (set `self.MainUI` _returnvalue_2))
      (`UserWidget.AddToViewport` _output_get 0)
      (`WidgetBlueprintLibrary.SetInputMode_UIOnlyEx` self (`self.MainUI`))
      (set `self.bShowMouseCursor` true))
    (:`then_1`
      ;[1 1 1] Bind to HTTP Events
      (add `HTTPSubsystem.OnTextResponse` _returnvalue (delegate `OnHttp_ResponseText`))
      (add `HTTPSubsystem.OnDataResponse` _returnvalue (delegate `OnHttp_ResponseData`))
      (add `HTTPSubsystem.OnResponseError` _returnvalue (delegate `OnHttp_Error`)))))

(event `OnHttp_ResponseData`
  (params (RequestName :type "Name (by ref)") (Code :type Integer) (Headers :type "Array of String (by ref)") (Data :type "Array of Byte (by ref)"))
  ;[1 1 1] Bind to HTTP Events
)

(event `OnHttp_ResponseText`
  (params (RequestName :type "Name (by ref)") (Code :type Integer) (Headers :type "Array of String (by ref)") (Data :type String))
  ;[1 1 1] Process data returned via HTTP
  (switch `/Game/Blueprins/E_State` (`self.State`)
    (:`NewEnumerator1`
      ;;[0.4461 1 0.4314] Text is Ready. Do Voice.
      (bind _output_get (set `self.NewTextToSpeak` (`JsonItemFunctionsLibrary.JsonGetFieldValue_String` (`JsonItemFunctionsLibrary.JsonItemFromString` Data) "choices[index=0].message.content")))
      (`self.SubmitTTSRequest` _output_get))
    (:`NewEnumerator2`
      ;;[0.08239 0.2273 1] Voice is Ready. Play It.
      (`self.Speak` (`JsonItemFunctionsLibrary.JsonGetFieldValue_String` (`JsonItemFunctionsLibrary.JsonItemFromString` Data) "data[1].path")))
    (:`NewEnumerator3`
      (`self.SetGenerationState` "NewEnumerator0"))))

(event `OnHttp_Error`
  (params (RequestName :type "Name (by ref)") (Code :type Integer))
  ;[1 1 1] Processing Errors
  (`|ExecutionSequence`
    (:`then_0`
      (switch `/Game/Blueprins/E_State` (`self.State`)
        (:`NewEnumerator1`
          (`KismetSystemLibrary.PrintString` "Couldn't generate text data"))
        (:`NewEnumerator2`
          (`KismetSystemLibrary.PrintString` "Couldn't generate audio data"))
        (:`NewEnumerator3`
          (`KismetSystemLibrary.PrintString` "Couldn't read audio file"))))
    (:`then_1`
      (`self.SetGenerationState` "NewEnumerator0"))))

(event `SubmitNewPrompt`
  (params (Text :type String))
  ;[1 0.3958 0.3958] Generate Text
  (switch `/Game/Blueprins/E_State` (`self.State`)
    (:`NewEnumerator0`
      (`self.SetGenerationState` "NewEnumerator1")
      (bind _output_get (set `self.CurrentRequest` (`JsonItemFunctionsLibrary.JsonItemFromString` (`self.Template_OpenAI`))))
      (`JsonItemFunctionsLibrary.JsonSetFieldValue_String` _output_get "messages[role=user].content" Text)
      (`HTTPSubsystem.SendHttpRequest` (subsystem `HTTPSubsystem`) "OpenAI" "http://127.0.0.1:1234/v1/chat/completions" "Post" (`|MakeArray` (`JsonItemFunctionsLibrary.GetDefaultContentAppJson`)) (`JsonItemFunctionsLibrary.JsonItemToString` (`self.CurrentRequest`)) "Default"))))

(event `SubmitTTSRequest`
  (params (Text :type String))
  ;[0.4461 1 0.4314] Generate Voice
  (switch `/Game/Blueprins/E_State` (`self.State`)
    (:`NewEnumerator1`
      (`self.SetGenerationState` "NewEnumerator2")
      (set `self.CurrentRequest` (`JsonItemFunctionsLibrary.JsonItemFromString` (`self.Template_TTS`)))
      (`JsonItemFunctionsLibrary.JsonSetFieldValue_String` (`self.CurrentRequest`) "data[2]" (`KismetStringLibrary.Concat_StrStr` (`KismetSystemLibrary.GetProjectDirectory`) "voice_ref.wav"))
      (`JsonItemFunctionsLibrary.JsonSetFieldValue_String` (`self.CurrentRequest`) "data[1]" Text)
      (`HTTPSubsystem.SendHttpRequest` (subsystem `HTTPSubsystem`) "TTS" "http://localhost:5003/run/run_tts" "Post" (`|MakeArray` (`JsonItemFunctionsLibrary.GetDefaultContentAppJson`)) (`JsonItemFunctionsLibrary.JsonItemToString` (`self.CurrentRequest`)) "Default"))))

(event `Speak`
  (params (AudioFIleName :type String))
  ;[0.08239 0.2273 1] Load and Play Generated Voice
  (`/Engine/EditorBlueprintResources/StandardMacros.IsValid` (`self.RAI`)
    (:`Is Valid`
      _)
    (:`Is Not Valid`
      (bind _returnvalue (`RuntimeAudioImporterLibrary.CreateRuntimeAudioImporter`))
      (bind _output_get (set `self.RAI` _returnvalue))
      (add `RuntimeAudioImporterLibrary.OnResult` _output_get (delegate `OnAudioFileLoaded`))))
  (`RuntimeAudioImporterLibrary.ImportAudioFromFile` (`self.RAI`) AudioFIleName "Wav"))

(event `OnAudioFileLoaded`
  (params (Importer :type "RuntimeAudioImporterLibrary Object Reference") (ImportedSoundWave :type "ImportedSoundWave Object Reference") (Status :type "ERuntimeImportStatus Enum" :default "SuccessfulImport"))
  ;[0.08239 0.2273 1] Load and Play Generated Voice
  (`self.SetGenerationState` "NewEnumerator3")
  (`/Game/Blueprins/BP_SpeakingHead.Speak` (`self.SpeakingHead`) ImportedSoundWave))

(fn `UserConstructionScript`)