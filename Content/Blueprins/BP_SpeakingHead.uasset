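; BP_SpeakingHead is a talking head that plays supplied audio with fake lip-sync on its skeletal mesh.
; It registers with BP_PlayerController on BeginPlay and plays sounds passed to Speak.
; Audio envelope values, shaped by a time-based sine pulse, drive morph target weights for visemes picked by real time rather than speech content.
; When audio finishes, it updates the controller's generation state to signal the phrase is over.
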(event `self.ReceiveBeginPlay`
  (bind _asbp_player_controller (cast `/Game/Blueprins/BP_PlayerController` (`GameplayStatics.GetPlayerController` 0)))
  (set `/Game/Blueprins/BP_PlayerController.SpeakingHead` self _asbp_player_controller))

(event `Speak`
  (params (AudioAsset :type "SoundBase Object Reference"))
  (bind _audio (`self.Audio`))
  (`AudioComponent.SetSound` _audio AudioAsset)
  (`AudioComponent.Play` _audio 0.0))

(event `self.Audio.OnAudioSingleEnvelopeValue`
  (params (PlayingSoundWave :type "SoundWave Object Reference") (EnvelopeValue :type "Float (single-precision)"))
  (bind _returnvalue (`GameplayStatics.GetRealTimeSeconds`))
  (bind _returnvalue_2 (/ 1.0 (`self.AnimationSpeed`)))
  ;[1 1 1] Fake lip-sync
  (bind _output_get (set `self.VisemeIndex` (`KismetMathLibrary.FTrunc` (mod _returnvalue (* _returnvalue_2 (`KismetArrayLibrary.Array_Length` (`self.Visemes`)))))))
  (`SkeletalMeshComponent.SetMorphTarget` (`self.SkeletalMesh`) (`|GetArrayItem` (`self.Visemes`) _output_get) (`KismetMathLibrary.FClamp` (* EnvelopeValue (`KismetMathLibrary.Sin` (* (/ (mod _returnvalue _returnvalue_2) _returnvalue_2) (`KismetMathLibrary.GetPI`))) 30.0)) true))

(event `self.Audio.OnAudioFinished`
  ;[1 1 1] Notify player controller that the phrase is finished
  (bind _asbp_player_controller (cast `/Game/Blueprins/BP_PlayerController` (`GameplayStatics.GetPlayerController` 0)))
  (`/Game/Blueprins/BP_PlayerController.SetGenerationState` _asbp_player_controller "NewEnumerator0"))

(fn `UserConstructionScript`)